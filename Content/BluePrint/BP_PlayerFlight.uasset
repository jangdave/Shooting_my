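; Player flight Blueprint for a shooter, whose event graph holds only inactive input wiring.
; Unconnected Enhanced Input nodes would add IMC_ShootingMapping and route action values to Horizental, Vertical, Boost and FireBullet, none of which are defined here.
; BeginPlay, overlap, Tick and the construction script are empty, so this graph runs no logic.
; Korean notes say the nodes work once connected, with fire using only the Triggered pin.
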(event `InputAction|Boost`
  (params (Key :type "Key Structure")))

(event `self.ReceiveBeginPlay`
  ;[1 1 1] 연결시 작동
)

(event `EnhancedInput|/Game/NewInput/IA_Horizental`
  (params (ActionValue :type "Float (double-precision)") (ElapsedSeconds :type "Float (double-precision)") (TriggeredSeconds :type "Float (double-precision)") (InputAction :type "InputAction Object Reference" :default "/Game/NewInput/IA_Horizental.IA_Horizental"))
  ;[1 1 1] 트리거, 컴플리트 연결시 작동 fire는 트리거만
)

(event `EnhancedInput|/Game/NewInput/IA_Vertical`
  (params (ActionValue :type "Float (double-precision)") (ElapsedSeconds :type "Float (double-precision)") (TriggeredSeconds :type "Float (double-precision)") (InputAction :type "InputAction Object Reference" :default "/Game/NewInput/IA_Vertical.IA_Vertical"))
  ;[1 1 1] 트리거, 컴플리트 연결시 작동 fire는 트리거만
)

(event `EnhancedInput|/Game/NewInput/IA_FireBullet`
  (params (ActionValue :type Boolean) (ElapsedSeconds :type "Float (double-precision)") (TriggeredSeconds :type "Float (double-precision)") (InputAction :type "InputAction Object Reference" :default "/Game/NewInput/IA_FireBullet.IA_FireBullet"))
  ;[1 1 1] 트리거, 컴플리트 연결시 작동 fire는 트리거만
)

(event `EnhancedInput|/Game/NewInput/IA_Boost`
  (params (ActionValue :type Boolean) (ElapsedSeconds :type "Float (double-precision)") (TriggeredSeconds :type "Float (double-precision)") (InputAction :type "InputAction Object Reference" :default "/Game/NewInput/IA_Boost.IA_Boost"))
  ;[1 1 1] 트리거, 컴플리트 연결시 작동 fire는 트리거만
)

(fn `UserConstructionScript`)